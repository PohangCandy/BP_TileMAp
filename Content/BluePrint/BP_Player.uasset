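; BP_Player is a player actor that steps across a clamped five-by-five grid, with separate logic for sliding along X.
; Move shifts a grid index by direction and snaps the actor to that cell.
; MovePlayer advances X by MoveSpeed and frame delta, and a BeginPlay timer zeroes that speed after one second.
; State-gated chains for moving and fighting call CallMoveEvent and CallFightEvent, but have no connected trigger.
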(event `self.ReceiveBeginPlay`
  (`KismetSystemLibrary.K2_SetTimerDelegate` (delegate `Player Stop`) 1.0))

(event `Player Stop`
  (set `self.MoveSpeed` 0.0))

(event `Key|Left`
  (params (Key :type "Key Structure")))

(event `Key|Right`
  (params (Key :type "Key Structure")))

(event `Key|Up`
  (params (Key :type "Key Structure")))

(event `Key|Down`
  (params (Key :type "Key Structure")))

(event `Key|SpaceBar`
  (params (Key :type "Key Structure")))

(event `Move Player`
  (bind (_returnvalue_x _returnvalue_y _returnvalue_z) (`KismetMathLibrary.BreakVector` (`self.K2_GetActorLocation`)))
  (`self.K2_SetActorLocation` (`KismetMathLibrary.MakeVector` (+ _returnvalue_x (* (`GameplayStatics.GetWorldDeltaSeconds`) (`self.MoveSpeed`))) _returnvalue_y _returnvalue_z)))

(fn `Move`
  (params (NewParam :type "/Game/Enum/EMove Enum" :default "NewEnumerator0") (NewParam1 :type Boolean))
  (switch `/Game/Enum/EMove` NewParam
    (:`NewEnumerator0`
      (bind _result (`/Engine/EditorBlueprintResources/StandardMacros.DecrementInt` (`self.IndexY`))
        (:`  `
          (set `self.IndexY` (`KismetMathLibrary.Clamp` _result 0 4)))))
    (:`NewEnumerator1`
      (bind _result_2 (`/Engine/EditorBlueprintResources/StandardMacros.IncrementInt` (`self.IndexY`))
        (:`  `
          (set `self.IndexY` (`KismetMathLibrary.Clamp` _result_2 0 4)))))
    (:`NewEnumerator2`
      (bind _result_3 (`/Engine/EditorBlueprintResources/StandardMacros.IncrementInt` (`self.IndexX`))
        (:`  `
          (set `self.IndexX` (`KismetMathLibrary.Clamp` _result_3 0 4)))))
    (:`NewEnumerator3`
      (bind _result_4 (`/Engine/EditorBlueprintResources/StandardMacros.DecrementInt` (`self.IndexX`))
        (:`  `
          (set `self.IndexX` (`KismetMathLibrary.Clamp` _result_4 0 4))))))
  (`self.K2_SetActorLocation` (`KismetMathLibrary.MakeVector` (* (`self.IndexX`) 100.0) (* (`self.IndexY`) 100.0))))

(fn `UserConstructionScript`)