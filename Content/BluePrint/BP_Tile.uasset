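; BP_Tile is a grid tile actor that can hold gold, an enemy and a trap.
; AdjustData derives grid coordinates from an array index five wide, writing X to itself and Y to the passed element, then rolls the contents through probability helpers.
; AdjustPos places the tile on a 100-unit grid from those coordinates, and TrapOn turns the ground material red.
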(fn `AdjustData`
  (params (ArrayElemants :type "/Game/BluePrint/BP_Tile Object Reference") (ArraryIndex :type Integer))
  (locals (NewLocalVar :type "/Game/BluePrint/BP_Tile Object Reference"))
  (`|ExecutionSequence`
    (:`then_0`
      (bind _output_get (set `self.LocalArrayElements` ArrayElemants))
      (bind _output_get_2 (set `self.LocalArraryIndex` ArraryIndex))
      (set `self.PositionX` (/ _output_get_2 5))
      (set `/Game/BluePrint/BP_Tile.PosxitionY` (mod _output_get_2 5) _output_get))
    (:`then_1`
      (bind _newparam1 (`/Game/Function/Test_Fuction_Lib.ProbCoin` 45 50))
      (set `self.Gold` _newparam1)
      (bind _newparam (`/Game/Function/Test_Fuction_Lib.ProbConfirm` 20))
      (set `self.bEnemyExist` _newparam)
      (set `self.bTrapExist` _newparam))))

(fn `AdjustPos`
  (`self.K2_SetActorLocation` (`KismetMathLibrary.MakeVector` (* (`self.PositionX`) 100.0) (* (`self.PosxitionY`) 100.0) 1.0)))

(fn `TrapOn`
  (`PrimitiveComponent.SetMaterial` (`self.Ground`) 0 "/Game/Material/M_Red.M_Red"))

(fn `UserConstructionScript`)