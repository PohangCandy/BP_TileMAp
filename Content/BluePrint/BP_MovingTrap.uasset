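; BP_MovingTrap is a trap actor that shuttles back and forth along the world Y axis.
; Tick reads TrapState and calls GoToForward or GoToBack, which set the state and offset the location by MoveSpeed scaled by delta time.
; Each event uses a one-second Delay before calling the opposite one to reverse direction.
; SetTimerByEvent nodes for the same switch are left unexecuted.
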(event `self.ReceiveTick`
  (params (DeltaSeconds :type "Float (single-precision)"))
  (switch `/Game/Enum/EMove` (`self.TrapState`)
    (:`NewEnumerator0`
      (`self.Go to forward`))
    (:`NewEnumerator1`
      (`self.Go to Back`))))

(event `Go to forward`
  (bind (_returnvalue_x _returnvalue_y _returnvalue_z) (`KismetMathLibrary.BreakVector` (`self.K2_GetActorLocation`)))
  (bind _output_get (set `self.TrapState` "NewEnumerator0"))
  (switch `/Game/Enum/EMove` _output_get
    (:`NewEnumerator0`
      (`self.K2_SetActorLocation` (`KismetMathLibrary.MakeVector` _returnvalue_x (+ _returnvalue_y (* (`GameplayStatics.GetWorldDeltaSeconds`) (`self.MoveSpeed`))) _returnvalue_z))
      (`KismetSystemLibrary.Delay` 1.0)
      (`self.Go to Back`))))

(event `Go to Back`
  (bind (_returnvalue_x _returnvalue_y _returnvalue_z) (`KismetMathLibrary.BreakVector` (`self.K2_GetActorLocation`)))
  (set `self.TrapState` "NewEnumerator1")
  (switch `/Game/Enum/EMove` (`self.TrapState`)
    (:`NewEnumerator1`
      (`self.K2_SetActorLocation` (`KismetMathLibrary.MakeVector` _returnvalue_x (+ _returnvalue_y (* (`GameplayStatics.GetWorldDeltaSeconds`) (`self.MoveSpeed`) -1.0)) _returnvalue_z))
      (`KismetSystemLibrary.Delay` 1.0)
      (`self.Go to forward`))))

(fn `UserConstructionScript`)